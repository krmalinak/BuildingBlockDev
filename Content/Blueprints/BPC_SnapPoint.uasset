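; BPC_SnapPoint is a scene component that acts as a snap point, pairing with another snap point and tracking that link.
; SnapPointTo stores the partner and calls back on it for a symmetric link, with IsSnapped guarding against endless recursion.
; BreakSnap clears its own link, but its nested call targets itself, leaving the partner's state unchanged.
; A helper sets the point's relative location; snapping itself moves nothing.
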(event `self.ReceiveTick`
  (params (DeltaSeconds :type "Float (single-precision)")))

(event `self.ReceiveInitializeComponent`)

(fn `BreakSnap`
  (bind _othersnappoint (`self.OtherSnapPoint`))
  (if (`self.IsSnapped`)
    (set `self.IsSnapped` false)
    (if (and (`KismetSystemLibrary.IsValid` _othersnappoint) (`/Game/Blueprints/BPC_SnapPoint.IsSnapped` _othersnappoint))
      (`self.BreakSnap`))
    (set `self.OtherSnapPoint` null)))

(fn `SetSnapPointRelativeLocation`
  (params (NewRelativeLocation :type "Object.Vector Structure" :default (0.0 0.0 0.0)))
  (`self.K2_SetRelativeLocation` NewRelativeLocation))

(fn `SnapPointTo`
  (params (OtherSnapPoint :type "/Game/Blueprints/BPC_SnapPoint Object Reference"))
  (if (not (`self.IsSnapped`))
    ;[1 1 1] set local vars
    (set `self.IsSnapped` true)
    (bind _output_get (set `self.OtherSnapPoint` OtherSnapPoint))
    ;[1 1 1] symmetric snap
    (if (not (`/Game/Blueprints/BPC_SnapPoint.IsSnapped` OtherSnapPoint))
      (`self.SnapPointTo` _output_get self))))