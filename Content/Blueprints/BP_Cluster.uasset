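; Cluster actor that owns a set of BP_BuildingBlock actors joined at snap points and attached to its root.
; BeginPlay spawns an initial block, then after a delay snaps six test blocks onto it using paired snap point indices.
; Attaching links both snap points and offsets the new block by their relative locations, copying the existing block's rotation.
; Detaching only breaks a block's snaps, and cluster-to-cluster merging is an unfinished stub.
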(event EventBeginPlay
  (bind _blocks (Variables|Default|GetBlocks))
  (bind _item (Utilities|Array|Get(acopy) _blocks))
  (bind _snappoints (Variables|/Game/Blueprints/BP_BuildingBlock.BP_BuildingBlock_C|GetSnapPoints _item))
  (Utilities|FlowControl|Sequence
    (:then_0
      ;[1 1 1] add initial block
      (Utilities|Array|Clear (Variables|Default|GetBlocks))
      (bind _returnvalue (Game|SpawnActorfromClass "/Game/Blueprints/BP_BuildingBlock.BP_BuildingBlock_C" (Transformation|GetActorTransform) true false self (Variables|Default|GetIsPhysicsEnabled) (Variables|Default|GetIsGravityEnabled)))
      (bind _output_get (Variables|Default|SetInitialBlock _returnvalue))
      (Class|Actor|AttachRootComponentto _output_get (Variables|Default|GetRoot) "None" "SnapToTarget" true)
      (Utilities|Array|Add (Variables|Default|GetBlocks) _returnvalue))
    (:then_1
      (Utilities|FlowControl|Delay 1.0)
      (Development|PrintString "Hello")
      (Utilities|FlowControl|Sequence
        (:then_0
          (Attachment|SpawnBlockandAttach (Utilities|Array|Get(acopy) _snappoints) 1))
        (:then_1
          (Attachment|SpawnBlockandAttach (Utilities|Array|Get(acopy) _snappoints 1)))
        (:then_2
          (Attachment|SpawnBlockandAttach (Utilities|Array|Get(acopy) _snappoints 2) 3))
        (:then_3
          (Attachment|SpawnBlockandAttach (Utilities|Array|Get(acopy) _snappoints 3) 2))
        (:then_4
          (Attachment|SpawnBlockandAttach (Utilities|Array|Get(acopy) _snappoints 4) 5))
        (:then_5
          (Attachment|SpawnBlockandAttach (Utilities|Array|Get(acopy) _snappoints 5) 4))))))

(fn ConstructionScript)

(fn AttachBlocktoCluster
  (params (ClusterSnapPoint :type BPC%20Snap%20Point%20Object%20Reference) (BlockSnapPoint :type BPC%20Snap%20Point%20Object%20Reference))
  (Utilities|FlowControl|Sequence
    (:then_0
      ;[1 1 1] update variables and attach to root
      (LocalVariables|SetClusterBlock (Variables|/Game/Blueprints/BPC_SnapPoint.BPC_SnapPoint_C|GetBuildingBlock ClusterSnapPoint))
      (bind _output_get (LocalVariables|SetNewBlock (Variables|/Game/Blueprints/BPC_SnapPoint.BPC_SnapPoint_C|GetBuildingBlock BlockSnapPoint)))
      (Class|Actor|AttachRootComponentto _output_get (Variables|Default|GetRoot) "None" "KeepRelativeOffset" true)
      (Utilities|Array|Add (Variables|Default|GetBlocks) _output_get))
    (:then_1
      ;[1 1 1] update BPC_SnapPoint variableas
      (Default|SnapPointto ClusterSnapPoint BlockSnapPoint))
    (:then_2
      ;[1 1 1] calculate relative location of new block
      (Utilities|FlowControl|Sequence
        (:then_0
          (bind _returnvalue (Transformation|GetRelativeTransform (LocalVariables|GetClusterBlock))))
        (:then_1
          (bind _returnvalue_2 (Transformation|GetRelativeTransform ClusterSnapPoint)))
        (:then_2
          (bind _returnvalue_3 (Transformation|GetRelativeTransform BlockSnapPoint))
          (Development|PrintString (Utilities|String|ToString(Vector) (.location _returnvalue_2)))
          (Transformation|SetActorRelativeTransform (LocalVariables|GetNewBlock) (Math|Transform|MakeTransform (+ (.location _returnvalue) (.location _returnvalue_2) (* (.location _returnvalue_3) -1.0)) (.rotation _returnvalue) "1.000000,1.000000,1.000000") false))))))

(fn SpawnBlockandAttach
  (params (ClusterPoint :type BPC%20Snap%20Point%20Object%20Reference) (BlockSnapPointIndex :type Integer :default 0))
  (bind _returnvalue (Game|SpawnActorfromClass "/Game/Blueprints/BP_BuildingBlock.BP_BuildingBlock_C" (Transformation|GetActorTransform) true true self (Variables|Default|GetIsPhysicsEnabled) (Variables|Default|GetIsGravityEnabled)))
  (Attachment|AttachBlocktoCluster ClusterPoint (Utilities|Array|Get(acopy) (Variables|/Game/Blueprints/BP_BuildingBlock.BP_BuildingBlock_C|GetSnapPoints _returnvalue) BlockSnapPointIndex)))

(fn AttachClustertoCluster
  (params (ThisSnapPoint :type BPC%20Snap%20Point%20Object%20Reference) (OtherSnapPoint :type BPC%20Snap%20Point%20Object%20Reference))
  ;[1 1 1] NB: this cluster persists, other cluster is destroyed
  (Utilities|FlowControl|Sequence
    (:then_0
      (LocalVariables|SetThisBlock (Variables|/Game/Blueprints/BPC_SnapPoint.BPC_SnapPoint_C|GetBuildingBlock ThisSnapPoint))
      (bind _output_get (LocalVariables|SetOtherBlock (Variables|/Game/Blueprints/BPC_SnapPoint.BPC_SnapPoint_C|GetBuildingBlock OtherSnapPoint)))
      (LocalVariables|SetOtherCluster (Variables|/Game/Blueprints/BP_BuildingBlock.BP_BuildingBlock_C|GetCluster _output_get)))
    (:then_1
      (for _array_element (Variables|BP_Cluster_C|GetBlocks (LocalVariables|GetOtherCluster))
        _))))

(fn DetachBlockfromCluster
  (params (BlockToFree :type BP%20Building%20Block%20Object%20Reference))
  (for _array_element (Variables|/Game/Blueprints/BP_BuildingBlock.BP_BuildingBlock_C|GetSnapPoints BlockToFree)
    (if (Variables|/Game/Blueprints/BPC_SnapPoint.BPC_SnapPoint_C|GetIsSnapped _array_element)
      (Default|BreakSnap _array_element))))