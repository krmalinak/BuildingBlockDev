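; BP_BuildingBlock is a building block with a configurable mesh, material and physics, plus a scaled overlay mesh for overlap detection.
; The construction script applies these settings; toggling collisions shows or hides the overlay, whose overlaps store another differently owned block as CollidingBlock.
; SetSnapPoints creates snap-point components from locations, but its construction call is disconnected.
; FindClosestSnapPoints compares two blocks' points by distance, returning inside the loop at the first match.
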(event OnComponentBeginOverlap(CollisionMesh)
  (params (OtherActor :type Actor%20Object%20Reference) (OtherComp :type Primitive%20Component%20Object%20Reference) (OtherBodyIndex :type Integer) (bFromSweep :type Boolean) (SweepResult :type Hit%20Result%20Structure%20%28by%20ref%29))
  (if (Math|Boolean|ANDBoolean (Variables|CollisionSettings|GetCollisionsEnabled) (!= OtherActor self) (!= (Components|GetOwner OtherActor) (Components|GetOwner (Variables|Default|GetRoot))) (== (Utilities|GetClass OtherActor) "BP_BuildingBlock_C"))
    (bind _asbp_building_block (Utilities|Casting|CastToBP_BuildingBlock OtherActor))
    (Variables|CollisionSettings|SetCollidingBlock _asbp_building_block)))

(event Custom|ToggleCollisions
  (params (EnableCollisions :type Boolean :default false))
  (CallFunction|SetCollisionSettings EnableCollisions))

(event EventTick
  (params (DeltaSeconds :type Float%20%28single-precision%29))
  (if (Variables|CollisionSettings|GetIsColliding)
    _))

(fn ConstructionScript
  (bind _blockmesh (Variables|Default|GetBlockMesh))
  (bind _blockstaticmesh (Variables|BlockMeshSettings|GetBlockStaticMesh))
  (bind _collisionmesh (Variables|Default|GetCollisionMesh))
  (bind _blockmesh_2 (Variables|Default|GetBlockMesh))
  (Utilities|FlowControl|Sequence
    (:then_0
      ;[1 1 1] init block and collision meshes
      (Components|StaticMesh|SetStaticMesh _blockmesh _blockstaticmesh)
      (Rendering|Material|SetMaterial _blockmesh 0 (Variables|BlockMeshSettings|GetBlockMaterial))
      (Components|StaticMesh|SetStaticMesh _collisionmesh _blockstaticmesh)
      (Rendering|Material|SetMaterial _collisionmesh 0 (Variables|CollisionSettings|GetCollisionMeshMaterial)))
    (:then_1
      ;[1 1 1] set physics settings
      (Physics|SetSimulatePhysics _blockmesh_2 (Variables|BlockMeshSettings|GetIsPhysicsEnabled))
      (Physics|SetEnableGravity _blockmesh_2 (Variables|BlockMeshSettings|GetIsGravityEnabled))
      (bind _returnvalue (Physics|GetCenterOfMass _blockmesh_2 "None"))
      (Variables|BlockMeshSettings|SetBlockCenter _returnvalue))
    (:then_2
      (CallFunction|SetCollisionSettings (Variables|CollisionSettings|GetCollisionsEnabled)))))

(fn SetSnapPoints
  (bind _snappointlocations (Variables|SnapPointSettings|GetSnapPointLocations))
  (Utilities|FlowControl|Sequence
    (:then_0
      (Utilities|Array|Clear (Variables|SnapPointSettings|GetSnapPoints))
      (for (_ _array_index) _snappointlocations
        (bind _returnvalue (AddComponent|AddBPCSnapPoint false (Math|Transform|MakeTransform (* (Utilities|Array|Get(acopy) _snappointlocations _array_index) 1e+02) "0, 0, 0" "1,1,1")))
        (Variables|/Game/Blueprints/BPC_SnapPoint.BPC_SnapPoint_C|SetBuildingBlock _returnvalue self)
        (Variables|/Game/Blueprints/BPC_SnapPoint.BPC_SnapPoint_C|SetIndex _returnvalue _array_index)
        (Utilities|Array|Add (Variables|SnapPointSettings|GetSnapPoints) _returnvalue)))))

(fn SetCollisionSettings
  (params (EnableCollisions :type Boolean :default false))
  (bind _collisionmesh (Variables|Default|GetCollisionMesh))
  (bind _collisionmesh_2 (Variables|Default|GetCollisionMesh))
  (Variables|CollisionSettings|SetCollisionsEnabled EnableCollisions)
  (Rendering|SetVisibility _collisionmesh EnableCollisions true)
  (Transformation|SetRelativeScale3D _collisionmesh (Math|Conversions|ToVector(Float) (Variables|CollisionSettings|GetCollisionMeshScale)))
  (if EnableCollisions
    (Collision|SetCollisionEnabled _collisionmesh_2 "QueryOnly")
    (Collision|SetCollisionObjectType _collisionmesh_2 "ECC_WorldStatic")
    (Collision|SetCollisionResponsetoAllChannels _collisionmesh_2 "ECR_Overlap")
    (else
      (Collision|SetCollisionEnabled _collisionmesh_2 "NoCollision")
      (Collision|SetCollisionObjectType _collisionmesh_2 "ECC_WorldStatic")
      (Collision|SetCollisionResponsetoAllChannels _collisionmesh_2 "ECR_Ignore"))))

(fn FindClosestSnapPoints
  (params (OtherBlock :type BP%20Building%20Block%20Object%20Reference))
  (for _array_element (Variables|BP_BuildingBlock_C|GetSnapPoints OtherBlock)
    (for _array_element_2 (Variables|SnapPointSettings|GetSnapPoints)
      (if (or (not (Utilities|IsValid (LocalVariables|GetThisSnapPoint))) (< (Math|Vector|VectorLength (- (Transformation|GetWorldLocation _array_element_2) (Transformation|GetWorldLocation _array_element))) (LocalVariables|GetMinimumDistance)))
        (LocalVariables|SetThisSnapPoint _array_element_2)
        (LocalVariables|SetOtherSnapPoint _array_element)
        (LocalVariables|SetMinimumDistance (Math|Vector|VectorLength (- (Transformation|GetWorldLocation _array_element_2) (Transformation|GetWorldLocation _array_element))))
        (return (LocalVariables|GetThisSnapPoint) (LocalVariables|GetOtherSnapPoint) (Math|Vector|VectorLength (- (Transformation|GetWorldLocation _array_element_2) (Transformation|GetWorldLocation _array_element))))))))